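; Kitchen stove fire hazard for VR fire training, extending a parent fire sample and lit on BeginPlay.
; Activating or deactivating the fire toggles two particle trails, audio and a query-only danger box.
; Powder and CO2 extinguishers trigger the hit behaviour, while Foam only shows a warning.
; A grasping hand entering the box triggers a one-time task failure, fading the camera out and returning to the Lobby.
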(event `self.ReceiveBeginPlay`
  (`parent.ReceiveBeginPlay`)
  (`self.Active Fire On Sample`))

(event `self.Active Fire On Sample`
  (`parent.Active Fire On Sample`)
  (`ParticleSystemComponent.BeginTrails` (`self.ParticleSystem`) "None" "None" "ETrailWidthMode_FromFirst" 0.0)
  (`ParticleSystemComponent.BeginTrails` (`self.ParticleSystem1`) "None" "None" "ETrailWidthMode_FromFirst" 0.0)
  (`AudioComponent.Play` (`self.Audio`) 0.0)
  (`PrimitiveComponent.SetCollisionEnabled` (`self.Box`) "QueryOnly"))

(event `self.Deactive Fire On Sample`
  (`parent.Deactive Fire On Sample`)
  (`ParticleSystemComponent.EndTrails` (`self.ParticleSystem`))
  (`ParticleSystemComponent.EndTrails` (`self.ParticleSystem1`))
  (`AudioComponent.Stop` (`self.Audio`))
  (`PrimitiveComponent.SetCollisionEnabled` (`self.Box`) "NoCollision"))

(event `self.Extinguished`
  (params (Type :type "/Game/FireTraining/Blueprints/Enums/E_Fireextinguisher Enum" :default "NewEnumerator0") (Target :type "Actor Object Reference"))
  (switch `/Game/FireTraining/Blueprints/Enums/E_Fireextinguisher` Type
    (:`NewEnumerator0`
      (`self.Warning` null "- Bình dạng bọt Foam \n- Bình khí nén CO2"))
    (:`NewEnumerator1`
      (`self.On Hit Behaviour` :!label _label))
    (:`NewEnumerator2`
      (goto _label))))

(event `self.Box.OnComponentBeginOverlap`
  (params (OverlappedComponent :type "PrimitiveComponent Object Reference") (OtherActor :type "Actor Object Reference") (OtherComp :type "PrimitiveComponent Object Reference") (OtherBodyIndex :type Integer) (bFromSweep :type Boolean) (SweepResult :type "HitResult Structure (by ref)"))
  (bind _asgrasping_hand (cast `/Game/VRExpansion/Vive/Testing/GraspingHand/GraspingHand` OtherActor))
  (bind _returnvalue (`self.GetOwner` _asgrasping_hand))
  (bind _asvive_pawn_character (cast `/Game/VRExpansion/Vive/Vive_PawnCharacter` _returnvalue))
  (`/Engine/EditorBlueprintResources/StandardMacros.DoOnce` false
    (:`Completed`
      (`/Game/VRExpansion/Vive/Vive_PawnCharacter.Show Notifycation` _asvive_pawn_character "/Game/FireTraining/Blueprints/Widgets/WBP_TaskFail.WBP_TaskFail_C")
      (bind _aspc_fire_training (cast `/Game/FireTraining/Framework/PC_FireTraining` (`self.GetOwner` _returnvalue)))
      (`PlayerCameraManager.StartCameraFade` :`self` (`GameplayStatics.GetPlayerCameraManager` (`GameplayStatics.GetPlayerControllerID` _aspc_fire_training)) :`ToAlpha` 1.0 :`Duration` 3.0 :`bShouldFadeAudio` true :`bHoldWhenFinished` true)
      (`KismetSystemLibrary.Delay` 3.0)
      (`GameplayStatics.OpenLevel` "Lobby"))))

(fn `UserConstructionScript`)