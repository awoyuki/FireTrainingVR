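; BP_FireBoxEquipment is a fire equipment box item in the fire training content, with a constraint-hinged door.
; It records the door's world rotation at BeginPlay.
; When the door is dropped with the physics constraint's Swing1 angle within 10 degrees of zero, the door snaps back to that stored rotation, so it closes cleanly.
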(event `self.ReceiveBeginPlay`
  (set `self.Relative Rotation` (`SceneComponent.K2_GetComponentRotation` (`self.Door`))))

(event `self.Door.OnDropped`
  (params (GrippingController :type "GripMotionControllerComponent Object Reference") (GripInformation :type "BPActorGripInformation Structure (by ref)") (bWasSocketed :type Boolean))
  (if (`KismetMathLibrary.NearlyEqual_FloatFloat` (`PhysicsConstraintComponent.GetCurrentSwing1` (`self.PhysicsConstraint`)) 0.0 10.0)
    (`SceneComponent.K2_SetWorldRotation` (`self.Door`) (`self.Relative Rotation`) false false)))

(fn `UserConstructionScript`)