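; VR fire-training lecture station that shows an image panel and presents a spawned grippable item.
; Pawn overlap with the zone toggles its active state, recoloring it green or red, animating the WBP_Lecture widget and playing a sound.
; On BeginPlay it sets the image and spawns the item, with a timeline lifting it and rotating Spawn1.
; Gripping stops the timeline and lets the button, while active, destroy and respawn the item.
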(event `self.Zone.OnComponentBeginOverlap`
  (params (OverlappedComponent :type "PrimitiveComponent Object Reference") (OtherActor :type "Actor Object Reference") (OtherComp :type "PrimitiveComponent Object Reference") (OtherBodyIndex :type Integer) (bFromSweep :type Boolean) (SweepResult :type "HitResult Structure (by ref)"))
  (bind _audio (`self.Audio`))
  (bind _asvive_pawn_character (cast `/Game/VRExpansion/Vive/Vive_PawnCharacter` OtherActor))
  (if (not (and (== OtherComp (`Character.CapsuleComponent` _asvive_pawn_character)) (`self.IsOn`)))
    (set `self.IsOn` true)
    (bind _returnvalue (`KismetMaterialLibrary.CreateDynamicMaterialInstance` "/Game/FireTraining/Materials/M_Zone.M_Zone"))
    (`MaterialInstanceDynamic.SetVectorParameterValue` _returnvalue "Color" (struct :`G` 0.2 :`A` 1.0))
    (`PrimitiveComponent.SetMaterial` (`self.Zone`) 0 _returnvalue)
    (`self.Play Widget Anim` (`self.Widget`) true)
    (`AudioComponent.SetSound` _audio "/Game/FireTraining/Audio/Visibility.Visibility")
    (`AudioComponent.Play` _audio 0.0)))

(event `self.Zone.OnComponentEndOverlap`
  (params (OverlappedComponent :type "PrimitiveComponent Object Reference") (OtherActor :type "Actor Object Reference") (OtherComp :type "PrimitiveComponent Object Reference") (OtherBodyIndex :type Integer))
  (bind _audio (`self.Audio`))
  (cast `/Game/VRExpansion/Vive/Vive_PawnCharacter` OtherActor)
  (if (`self.IsOn`)
    (set `self.IsOn` false)
    (bind _returnvalue (`KismetMaterialLibrary.CreateDynamicMaterialInstance` "/Game/FireTraining/Materials/M_Zone.M_Zone"))
    (`MaterialInstanceDynamic.SetVectorParameterValue` _returnvalue "Color" (struct :`R` 0.2 :`A` 1.0))
    (`PrimitiveComponent.SetMaterial` (`self.Zone`) 0 _returnvalue)
    (`self.Play Widget Anim` (`self.Widget`))
    (`AudioComponent.SetSound` _audio "/Game/FireTraining/Audio/Hidden.Hidden")
    (`AudioComponent.Play` _audio 0.0)))

(event `self.ReceiveBeginPlay`
  (bind _actor_new_location (`self.Actor New Location`))
  (bind (_returnvalue_location _returnvalue_rotation _returnvalue_scale) (`KismetMathLibrary.BreakTransform` (`SceneComponent.K2_GetComponentToWorld` (`self.Spawn`))))
  (`self.Set Lecture Image` (`self.Widget`) (`self.Image`))
  (bind _returnvalue (`GameplayStatics.GetActorOfClass` (`self.Spawn Actor`) :!label _label))
  (`/Engine/EditorBlueprintResources/StandardMacros.IsValid` _returnvalue
    (:`Is Valid`
      (`self.K2_DestroyActor` _returnvalue))
    (:`Is Not Valid`
      _))
  (set `self.Is Spawned` true)
  (bind _returnvalue_2 (`|SpawnActorFromClass` (`self.Spawn Actor`) (`KismetMathLibrary.MakeTransform` (+ _returnvalue_location (0.0 0.0 20.0)) _returnvalue_rotation _returnvalue_scale) "AlwaysSpawn" "OverrideRootScale" null null))
  (bind _asgrippable_static_mesh_actor (cast `GrippableStaticMeshActor` _returnvalue_2))
  (add `GrippableStaticMeshActor.OnGripped` _asgrippable_static_mesh_actor (delegate `OnGripped_Event_0`))
  (set `self.Actor New Location` (`self.K2_GetActorLocation` _returnvalue_2))
  (bind (_direction _value _rotation) (`Timeline|Timeline_0` :!via `PlayFromStart` :!label _label_2)
    (:`Update`
      (`self.K2_SetActorLocation` _returnvalue_2 (`KismetMathLibrary.VLerp` _actor_new_location (+ _actor_new_location (0.0 0.0 60.0)) _value) false false)
      (`SceneComponent.K2_SetRelativeRotation` (`self.Spawn1`) (`KismetMathLibrary.RLerp` (struct) (struct :`Roll` 125.0) _rotation) false false))))

(event `self.BPC_Button.ButtonPressed`
  (params (ButtonState :type Boolean))
  (if (and (`self.IsOn`) (not (`self.Is Spawned`)))
    (goto _label)))

(event `OnGripped_Event_0`
  (params (GrippingController :type "GripMotionControllerComponent Object Reference") (GripInformation :type "BPActorGripInformation Structure (by ref)"))
  (set `self.Is Spawned` false)
  (goto _label_2 :!via `Stop`))

(fn `Play Widget Anim`
  (params (Widget :type "WidgetComponent Object Reference") (Forward :type Boolean))
  (bind _aswbp_lecture (cast `/Game/FireTraining/Blueprints/Widgets/WBP_Lecture` (`WidgetComponent.GetUserWidgetObject` Widget)))
  (if Forward
    (bind _imageanim (`/Game/FireTraining/Blueprints/Widgets/WBP_Lecture.ImageAnim` _aswbp_lecture))
    (`UserWidget.PlayAnimationForward` _aswbp_lecture _imageanim 1.0 false)
    (else
      (`UserWidget.PlayAnimationReverse` _aswbp_lecture _imageanim 1.0 false))))

(fn `Set Lecture Image`
  (params (Widget :type "WidgetComponent Object Reference") (Image :type "Texture2D Object Reference"))
  (bind _aswbp_lecture (cast `/Game/FireTraining/Blueprints/Widgets/WBP_Lecture` (`WidgetComponent.GetUserWidgetObject` Widget)))
  (`Image.SetBrushFromTexture` (`/Game/FireTraining/Blueprints/Widgets/WBP_Lecture.Image_24` _aswbp_lecture) Image true))

(fn `UserConstructionScript`)