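; Level-selection field in a VR fire training game, where the player picks a kitchen-fire or electrical-fire scenario and walks in to load it.
; BeginPlay fills two Vietnamese training-area signs; each button sets MapToLoad, updates the current-selection sign and plays audio.
; The Vive pawn's capsule entering Box triggers, once, a warning, sound and camera fade, then opens the map after a delay.
; Box1 shows a one-time introduction notification when ShowInstruction is set.
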(event `self.ReceiveBeginPlay`
  (`|ExecutionSequence`
    (:`then_0`
      (bind _aswbp_training_sign (cast `/Game/FireTraining/Blueprints/Widgets/WBP_TrainingSign` (`WidgetComponent.GetUserWidgetObject` (`self.Widget`))))
      (`TextBlock.SetText` (`/Game/FireTraining/Blueprints/Widgets/WBP_TrainingSign.Title` _aswbp_training_sign) "Khu vực tập huấn 01")
      (`TextBlock.SetText` (`/Game/FireTraining/Blueprints/Widgets/WBP_TrainingSign.Content` _aswbp_training_sign) "Thực hành xử lý tình huống cháy bếp tại nhà bếp."))
    (:`then_1`
      (bind _aswbp_training_sign_2 (cast `/Game/FireTraining/Blueprints/Widgets/WBP_TrainingSign` (`WidgetComponent.GetUserWidgetObject` (`self.Widget1`))))
      (`TextBlock.SetText` (`/Game/FireTraining/Blueprints/Widgets/WBP_TrainingSign.Title` _aswbp_training_sign_2) "Khu vực tập huấn 02")
      (`TextBlock.SetText` (`/Game/FireTraining/Blueprints/Widgets/WBP_TrainingSign.Content` _aswbp_training_sign_2) "Thực hành xử lý tình huống sự cố điện tại nhà bếp."))))

(event `self.Kitchen.ButtonPressed`
  (params (ButtonState :type Boolean))
  (if ButtonState
    (set `self.MapToLoad` "Kitchen")
    (bind _aswbp_training_sign_current (cast `/Game/FireTraining/Blueprints/Widgets/WBP_TrainingSignCurrent` (`WidgetComponent.GetUserWidgetObject` (`self.Widget2`))))
    (`TextBlock.SetText` (`/Game/FireTraining/Blueprints/Widgets/WBP_TrainingSignCurrent.Content` _aswbp_training_sign_current) "Thực hành xử lý tình huống cháy bếp tại nhà bếp.")
    (`AudioComponent.Play` (`self.Audio`) 0.0 :!label _label)))

(event `self.Electric.ButtonPressed`
  (params (ButtonState :type Boolean))
  (if ButtonState
    (set `self.MapToLoad` "Electric")
    (bind _aswbp_training_sign_current (cast `/Game/FireTraining/Blueprints/Widgets/WBP_TrainingSignCurrent` (`WidgetComponent.GetUserWidgetObject` (`self.Widget2`))))
    (`TextBlock.SetText` (`/Game/FireTraining/Blueprints/Widgets/WBP_TrainingSignCurrent.Content` _aswbp_training_sign_current) "Thực hành xử lý tình huống sự cố cháy điện tại nhà bếp.")
    (goto _label)))

(event `self.Box.OnComponentBeginOverlap`
  (params (OverlappedComponent :type "PrimitiveComponent Object Reference") (OtherActor :type "Actor Object Reference") (OtherComp :type "PrimitiveComponent Object Reference") (OtherBodyIndex :type Integer) (bFromSweep :type Boolean) (SweepResult :type "HitResult Structure (by ref)"))
  (bind _asvive_pawn_character (cast `/Game/VRExpansion/Vive/Vive_PawnCharacter` OtherActor))
  (if (== (`Character.CapsuleComponent` _asvive_pawn_character) OtherComp)
    (bind _aspc_fire_training (cast `/Game/FireTraining/Framework/PC_FireTraining` (`self.GetOwner` _asvive_pawn_character)))
    (`/Engine/EditorBlueprintResources/StandardMacros.DoOnce` false
      (:`Completed`
        (`/Game/VRExpansion/Vive/Vive_PawnCharacter.Show Notifycation` _asvive_pawn_character "/Game/FireTraining/Blueprints/Widgets/WBP_EnterTrainingWarning.WBP_EnterTrainingWarning_C")
        (`AudioComponent.Play` (`self.Audio1`) 0.0)
        (`PlayerCameraManager.StartCameraFade` :`self` (`GameplayStatics.GetPlayerCameraManager` (`AdvancedSessionsLibrary.GetNetPlayerIndex` _aspc_fire_training)) :`ToAlpha` 1.0 :`Duration` 3.0 :`bShouldFadeAudio` true :`bHoldWhenFinished` true)
        (`KismetSystemLibrary.Delay` 3.0)
        (`GameplayStatics.OpenLevel` (`self.MapToLoad`))))))

(event `self.Box1.OnComponentBeginOverlap`
  (params (OverlappedComponent :type "PrimitiveComponent Object Reference") (OtherActor :type "Actor Object Reference") (OtherComp :type "PrimitiveComponent Object Reference") (OtherBodyIndex :type Integer) (bFromSweep :type Boolean) (SweepResult :type "HitResult Structure (by ref)"))
  (bind _asvive_pawn_character (cast `/Game/VRExpansion/Vive/Vive_PawnCharacter` OtherActor))
  (if (and (== (`Character.CapsuleComponent` _asvive_pawn_character) OtherComp) (`self.ShowInstruction`))
    (`/Engine/EditorBlueprintResources/StandardMacros.DoOnce` false
      (:`Completed`
        (`/Game/VRExpansion/Vive/Vive_PawnCharacter.Show Notifycation` _asvive_pawn_character "/Game/FireTraining/Blueprints/Widgets/WBP_Introduction_04.WBP_Introduction_04_C")))))

(fn `UserConstructionScript`)