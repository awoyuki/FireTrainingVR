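; Flammable item for a fire training game, tracking the fire as a health value and able to show warnings to the player.
; Igniting restores full health; each hit removes one point and deactivates the fire at zero.
; Warning shows a WBP_FEWarning notification with custom text on the Vive pawn, gated by DoOnce until that notification is removed.
; The Extinguished event is an empty stub here.
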(event `/Game/FireTraining/Blueprints/Interfaces/BPI_Sample.Active Fire On Sample`
  (set `self.Health` (`self.MaxHealth`)))

(event `/Game/FireTraining/Blueprints/Interfaces/BPI_Sample.Deactive Fire On Sample`
  (set `self.Health` 0))

(event `Extinguished`
  (params (Type :type "/Game/FireTraining/Blueprints/Enums/E_Fireextinguisher Enum" :default "NewEnumerator0") (Target :type "Actor Object Reference")))

(event `Warning`
  (params (`Actor Cause` :type "Actor Object Reference") (InText :type Text))
  (`/Engine/EditorBlueprintResources/StandardMacros.DoOnce` false :!label _label
    (:`Completed`
      (bind _asvive_pawn_character (cast `/Game/VRExpansion/Vive/Vive_PawnCharacter` `Actor Cause`))
      (bind _returnvalue (`/Game/VRExpansion/Vive/Vive_PawnCharacter.Show Notifycation` _asvive_pawn_character "/Game/FireTraining/Blueprints/Widgets/WBP_FEWarning.WBP_FEWarning_C"))
      (add `/Game/FireTraining/Blueprints/Widgets/WBP_UI.On Disable Notify` (`/Game/VRExpansion/Vive/Vive_PawnCharacter.As WBP UI` _asvive_pawn_character) (delegate `CustomEvent_0`))
      (bind _aswbp_fewarning (cast `/Game/FireTraining/Blueprints/Widgets/WBP_FEWarning` _returnvalue))
      (`TextBlock.SetText` (`/Game/FireTraining/Blueprints/Widgets/WBP_FEWarning.TextBlock` _aswbp_fewarning) InText))))

(event `CustomEvent_0`
  (params (Removed :type "Widget Object Reference"))
  (if (== (stale `Warning` _returnvalue) Removed)
    (remove `/Game/FireTraining/Blueprints/Widgets/WBP_UI.On Disable Notify` (`/Game/VRExpansion/Vive/Vive_PawnCharacter.As WBP UI` (stale `Warning` _asvive_pawn_character)) (delegate `CustomEvent_0`))
    (goto _label :!via `Reset`)))

(fn `On Hit Behaviour`
  (bind _result (`/Engine/EditorBlueprintResources/StandardMacros.DecrementInt` (`self.Health`))
    (:`  `
      (if (<= _result 0)
        (set `self.Health` 0)
        (`/Game/FireTraining/Blueprints/Interfaces/BPI_Sample.Deactive Fire On Sample`)))))

(fn `UserConstructionScript`)