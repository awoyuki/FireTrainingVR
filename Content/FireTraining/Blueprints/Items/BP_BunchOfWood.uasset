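; BP_BunchOfWood is a burnable wood-pile item for a fire extinguisher training game.
; It extends parent fire activation and deactivation by toggling particle trails and looping fire audio.
; On extinguishing, Foam and Powder run the hit behaviour, while CO2 shows a Vietnamese warning naming foam and dry powder extinguishers as the suitable types.
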(event `/Game/FireTraining/Blueprints/Interfaces/BPI_Sample.Active Fire On Sample`
  (`parent.Active Fire On Sample`)
  (`ParticleSystemComponent.BeginTrails` (`self.ParticleSystem`) "None" "None" "ETrailWidthMode_FromFirst" 0.0)
  (`AudioComponent.Play` (`self.Audio`) 0.0))

(event `/Game/FireTraining/Blueprints/Interfaces/BPI_Sample.Deactive Fire On Sample`
  (`parent.Deactive Fire On Sample`)
  (`ParticleSystemComponent.EndTrails` (`self.ParticleSystem`))
  (`AudioComponent.Stop` (`self.Audio`)))

(event `self.Extinguished`
  (params (Type :type "/Game/FireTraining/Blueprints/Enums/E_Fireextinguisher Enum" :default "NewEnumerator0") (Target :type "Actor Object Reference"))
  (switch `/Game/FireTraining/Blueprints/Enums/E_Fireextinguisher` Type
    (:`NewEnumerator0`
      (`self.On Hit Behaviour` :!label _label))
    (:`NewEnumerator1`
      (goto _label))
    (:`NewEnumerator2`
      (`self.Warning` Target "- Bình dạng bọt Foam \n- Bình bột khô Powder"))))

(fn `UserConstructionScript`)