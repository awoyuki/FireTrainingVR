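; A grippable CO2 fire extinguisher for fire training that only fires once its safety cone is pulled clear of the capsule.
; Returning the held cone to the capsule drops, snaps and reattaches it, while custom depth highlights the cone or handle.
; Using it plays audio, Niagara spray and a handle animation while repeated line traces notify flammable objects or send other hit actors an extinguished message.
; Releasing the grip stops firing and locks the cone.
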(event `self.Capsule.OnComponentBeginOverlap`
  (params (OverlappedComponent :type "PrimitiveComponent Object Reference") (OtherActor :type "Actor Object Reference") (OtherComp :type "PrimitiveComponent Object Reference") (OtherBodyIndex :type Integer) (bFromSweep :type Boolean) (SweepResult :type "HitResult Structure (by ref)"))
  (bind _safetycone (`self.SafetyCone`))
  (bind (_returnvalue_location _returnvalue_rotation) (`KismetMathLibrary.BreakTransform` (`SceneComponent.K2_GetComponentToWorld` (`self.Capsule`))))
  (if (== OtherComp (`self.SafetyCone`))
    (bind _holdingcontrollers (`VRGripInterface.IsHeld` (`self.SafetyCone`)))
    (bind (_holdingcontroller _gripid) (break `BPGripPair` (`|GetArrayItem` _holdingcontrollers)))
    (`/Engine/EditorBlueprintResources/StandardMacros.IsValid` _holdingcontroller
      (:`Is Valid`
        (`GripMotionControllerComponent.DropObjectByInterface` _holdingcontroller (`self.SafetyCone`) _gripid (0.0 0.0 0.0) (0.0 0.0 0.0))
        (`PrimitiveComponent.SetSimulatePhysics` _safetycone false)
        (`KismetSystemLibrary.Delay` 0.1)
        (`SceneComponent.K2_SetWorldLocationAndRotation` _safetycone _returnvalue_location _returnvalue_rotation false true)
        (`SceneComponent.K2_AttachToComponent` (`self.SafetyCone`) (`self.StaticMeshComponent`) "None" "KeepWorld" "KeepWorld" "KeepWorld" true)
        (set `self.SafetyConeCheck` false)
        (`VRGripInterface.OnEndUsed`)
        (`PrimitiveComponent.SetRenderCustomDepth` (`self.SafetyCone`) (not (`self.SafetyConeCheck`)))))))

(event `self.SafetyCone.OnGripped`
  (params (GrippingController :type "GripMotionControllerComponent Object Reference") (GripInformation :type "BPActorGripInformation Structure (by ref)"))
  (bind _safetyconecheck (`self.SafetyConeCheck`))
  (if (`PrimitiveComponent.IsOverlappingComponent` (`self.SafetyCone`) (`self.Capsule`)) :!label _label
    (`KismetSystemLibrary.Delay` 0.2)
    (goto _label)
    (else
      (set `self.SafetyConeCheck` true)
      (`PrimitiveComponent.SetRenderCustomDepth` (`self.SafetyCone`) (not _safetyconecheck))
      (`PrimitiveComponent.SetRenderCustomDepth` (`self.Handle`) _safetyconecheck))))

(event `VRGripInterface.OnUsed`
  (bind _arrow (`self.Arrow`))
  (bind _returnvalue (`SceneComponent.K2_GetComponentLocation` _arrow))
  (if (`self.SafetyConeCheck`)
    (`AudioComponent.Play` (`self.Audio`) 0.0)
    (`PrimitiveComponent.SetRenderCustomDepth` (`self.Handle`) false)
    (set `self.Firing` true)
    (`NiagaraComponent.SetVariableFloat` (`self.Fire Niagara`) "Spawn Rate" 200.0)
    (`self.Play Handle Anim`)
    (if (`self.Firing`) :!label _label_2
      (bind _outhit (`KismetSystemLibrary.LineTraceSingle` _returnvalue (+ _returnvalue (* (`SceneComponent.GetForwardVector` _arrow) (`self.Distance`))) "TraceTypeQuery1"))
      (bind (_bblockinghit _binitialoverlap _time _distance _location _impactpoint _normal _impactnormal _physmat _hitactor _hitcomponent) (`GameplayStatics.BreakHitResult` _outhit))
      (`self.Get Hit Behaviour` _hitactor _hitcomponent)
      (`KismetSystemLibrary.RetriggerableDelay` (`self.Fire Rate`))
      (goto _label_2))))

(event `Play Handle Anim`
  (bind (_direction _value) (`Timeline|Lerp Rotation` :!via `PlayFromStart` :!label _label_3)
    (:`Update`
      (`SceneComponent.K2_SetRelativeRotation` (`self.Handle`) (`KismetMathLibrary.RLerp` (struct) (struct :`Pitch` -20.0) _value true) false false))))

(event `VRGripInterface.OnEndUsed`
  (`PrimitiveComponent.SetRenderCustomDepth` (`self.Handle`) (`self.SafetyConeCheck`))
  (set `self.Firing` false :!label _label_4)
  (`AudioComponent.Stop` (`self.Audio`))
  (`NiagaraComponent.SetVariableFloat` (`self.Fire Niagara`) "Spawn Rate" 0.0)
  (goto _label_3 :!via `Reverse`))

(event `VRGripInterface.OnGripRelease`
  (params (ReleasingController :type "GripMotionControllerComponent Object Reference") (GripInformation :type "BPActorGripInformation Structure (by ref)") (bWasSocketed :type Boolean))
  (`GrippableStaticMeshComponent.SetDenyGripping` (`self.SafetyCone`) true)
  (`PrimitiveComponent.SetRenderCustomDepth` (`self.SafetyCone`) false)
  (`PrimitiveComponent.SetRenderCustomDepth` (`self.Handle`) false)
  (goto _label_4))

(event `VRGripInterface.OnGrip`
  (params (GrippingController :type "GripMotionControllerComponent Object Reference") (GripInformation :type "BPActorGripInformation Structure (by ref)"))
  (bind _safetycone (`self.SafetyCone`))
  (bind _safetyconecheck (`self.SafetyConeCheck`))
  (`GrippableStaticMeshComponent.SetDenyGripping` _safetycone false)
  (`PrimitiveComponent.SetRenderCustomDepth` _safetycone (not _safetyconecheck))
  (`PrimitiveComponent.SetRenderCustomDepth` (`self.Handle`) _safetyconecheck))

(fn `Get Hit Behaviour`
  (params (`Actor Hit` :type "Actor Object Reference") (`Component Hit` :type "PrimitiveComponent Object Reference"))
  (bind _asbp_flammable_object (cast `/Game/FireTraining/Blueprints/Props/BP_FlammableObject` `Actor Hit`)
    (:`then`
      (`/Game/FireTraining/Blueprints/Props/BP_FlammableObject.On Extinguisher` _asbp_flammable_object `Component Hit`))
    (:`CastFailed`
      (message `/Game/FireTraining/Blueprints/Interfaces/BPI_Sample.Extinguished` `Actor Hit` (`self.Model`)))))

(fn `UserConstructionScript`)