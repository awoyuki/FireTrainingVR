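; Grippable fire extinguisher for fire training that puts out flammable objects while in use.
; Using it turns on the Niagara spray, rotates the handle via a timeline and repeats a forward line trace from an arrow at the fire rate, printing each hit.
; Hits on BP_FlammableObject call its OnExtinguisher with the struck component.
; Ending use or releasing the grip stops the spray and reverses the handle; the safety cone overlap has no effect yet.
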(event `self.ReceiveBeginPlay`
  (set `self.Bolt Relative Transform` (`SceneComponent.GetRelativeTransform` (`self.SafetyCone`))))

(event `self.SafetyCone.OnComponentBeginOverlap`
  (params (OverlappedComponent :type "PrimitiveComponent Object Reference") (OtherActor :type "Actor Object Reference") (OtherComp :type "PrimitiveComponent Object Reference") (OtherBodyIndex :type Integer) (bFromSweep :type Boolean) (SweepResult :type "HitResult Structure (by ref)"))
  (if (== OtherComp (`self.Capsule`))
    _))

(event `VRGripInterface.OnUsed`
  (bind _arrow (`self.Arrow`))
  (bind _returnvalue (`SceneComponent.K2_GetComponentLocation` _arrow))
  (set `self.Firing` true)
  (`NiagaraComponent.SetVariableFloat` (`self.Fire Niagara`) "Spawn Rate" 600.0)
  (`self.Play Handle Anim`)
  (if (`self.Firing`) :!label _label
    (bind _outhit (`KismetSystemLibrary.LineTraceSingle` _returnvalue (+ _returnvalue (* (`SceneComponent.GetForwardVector` _arrow) (`self.Distance`))) "TraceTypeQuery1"))
    (bind (_bblockinghit _binitialoverlap _time _distance _location _impactpoint _normal _impactnormal _physmat _hitactor _hitcomponent) (`GameplayStatics.BreakHitResult` _outhit))
    (`KismetSystemLibrary.PrintString` (`KismetStringLibrary.Concat_StrStr` "Actor: " (`KismetSystemLibrary.GetDisplayName` _hitactor) "Component:" (`KismetSystemLibrary.GetDisplayName` _hitcomponent)))
    (`self.Get Hit Behaviour` _hitactor _hitcomponent)
    (`KismetSystemLibrary.RetriggerableDelay` (`self.Fire Rate`))
    (goto _label)))

(event `Play Handle Anim`
  (bind (_direction _value) (`Timeline|Lerp Rotation` :!via `PlayFromStart` :!label _label_2)
    (:`Update`
      (`SceneComponent.K2_SetRelativeRotation` (`self.Handle`) (`KismetMathLibrary.RLerp` (struct) (struct :`Pitch` -20.0) _value true) false false))))

(event `VRGripInterface.OnEndUsed`
  (set `self.Firing` false :!label _label_3)
  (`NiagaraComponent.SetVariableFloat` (`self.Fire Niagara`) "Spawn Rate" 0.0)
  (goto _label_2 :!via `Reverse`))

(event `VRGripInterface.OnGripRelease`
  (params (ReleasingController :type "GripMotionControllerComponent Object Reference") (GripInformation :type "BPActorGripInformation Structure (by ref)") (bWasSocketed :type Boolean))
  (goto _label_3))

(fn `Get Hit Behaviour`
  (params (`Actor Hit` :type "Actor Object Reference") (`Component Hit` :type "PrimitiveComponent Object Reference"))
  (bind _asbp_flammable_object (cast `/Game/FireTraining/Blueprints/Props/BP_FlammableObject` `Actor Hit`))
  (`/Game/FireTraining/Blueprints/Props/BP_FlammableObject.On Extinguisher` _asbp_flammable_object `Component Hit`))

(fn `UserConstructionScript`)