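; BP_AlarmButton is a pressable button in the fire training game that turns off a referenced fire alarm.
; On BeginPlay it sets its widget component's WBP_Text to a Vietnamese "press to turn off the fire alarm" prompt, then hides it.
; Pressing ButtonTop calls DeactiveAlarm on the Alarm reference if valid and hides the prompt.
; Nothing in this Blueprint makes the prompt visible again.
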(event `self.ReceiveBeginPlay`
  (bind _aswbp_text (cast `/Game/FireTraining/Blueprints/Widgets/WBP_Text` (`WidgetComponent.GetUserWidgetObject` (`self.Widget`))))
  (`TextBlock.SetText` (`/Game/FireTraining/Blueprints/Widgets/WBP_Text.TextBlock_0` _aswbp_text) "Nhấn để tắt chuông báo cháy")
  (`SceneComponent.SetVisibility` (`self.Widget`) false false))

(event `self.ButtonTop.ButtonPressed`
  (params (ButtonState :type Boolean))
  (bind _alarm (`self.Alarm`)
    (:`then`
      (`/Game/FireTraining/Blueprints/Interfaces/BPI_Sample.Deactive Alarm` _alarm)
      (`SceneComponent.SetVisibility` (`self.Widget`) false false))
    (:`else`)))

(fn `UserConstructionScript`)