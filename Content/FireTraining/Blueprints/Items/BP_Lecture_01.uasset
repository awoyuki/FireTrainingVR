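; BP_Lecture_01 is a fire-training lecture station that reveals three image panels when a Vive pawn enters its zone.
; BeginPlay assigns textures to three WBP_Lecture widgets and resets the text's world rotation.
; Zone overlaps toggle IsOn, tint the zone green or red through new dynamic materials, and play show or hide sounds.
; A shared helper plays each widget's ImageAnim forward on entry and in reverse on exit.
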(event `self.ReceiveBeginPlay`
  (`self.Set Lecture Image` (`self.Widget`) (`self.Image`))
  (`self.Set Lecture Image` (`self.Widget1`) (`self.Image_0`))
  (`self.Set Lecture Image` (`self.Widget2`) (`self.Image_1`))
  (`SceneComponent.K2_SetWorldRotation` :`self` (`self.Text`)))

(event `self.Zone.OnComponentBeginOverlap`
  (params (OverlappedComponent :type "PrimitiveComponent Object Reference") (OtherActor :type "Actor Object Reference") (OtherComp :type "PrimitiveComponent Object Reference") (OtherBodyIndex :type Integer) (bFromSweep :type Boolean) (SweepResult :type "HitResult Structure (by ref)"))
  (bind _audio (`self.Audio`))
  (bind _asvive_pawn_character (cast `/Game/VRExpansion/Vive/Vive_PawnCharacter` OtherActor))
  (if (not (and (== OtherComp (`Character.CapsuleComponent` _asvive_pawn_character)) (`self.IsOn`)))
    (set `self.IsOn` true)
    (bind _returnvalue (`KismetMaterialLibrary.CreateDynamicMaterialInstance` "/Game/FireTraining/Materials/M_Zone.M_Zone"))
    (`MaterialInstanceDynamic.SetVectorParameterValue` _returnvalue "Color" (struct :`G` 0.2 :`A` 1.0))
    (`PrimitiveComponent.SetMaterial` (`self.Zone`) 0 _returnvalue)
    (`self.Play Widget Anim` (`self.Widget`) true)
    (`self.Play Widget Anim` (`self.Widget1`) true)
    (`self.Play Widget Anim` (`self.Widget2`) true)
    (`AudioComponent.SetSound` _audio "/Game/FireTraining/Audio/Visibility.Visibility")
    (`AudioComponent.Play` _audio 0.0)))

(event `self.Zone.OnComponentEndOverlap`
  (params (OverlappedComponent :type "PrimitiveComponent Object Reference") (OtherActor :type "Actor Object Reference") (OtherComp :type "PrimitiveComponent Object Reference") (OtherBodyIndex :type Integer))
  (bind _audio (`self.Audio`))
  (cast `/Game/VRExpansion/Vive/Vive_PawnCharacter` OtherActor)
  (if (`self.IsOn`)
    (set `self.IsOn` false)
    (bind _returnvalue (`KismetMaterialLibrary.CreateDynamicMaterialInstance` "/Game/FireTraining/Materials/M_Zone.M_Zone"))
    (`MaterialInstanceDynamic.SetVectorParameterValue` _returnvalue "Color" (struct :`R` 0.2 :`A` 1.0))
    (`PrimitiveComponent.SetMaterial` (`self.Zone`) 0 _returnvalue)
    (`self.Play Widget Anim` (`self.Widget`))
    (`self.Play Widget Anim` (`self.Widget1`))
    (`self.Play Widget Anim` (`self.Widget2`))
    (`AudioComponent.SetSound` _audio "/Game/FireTraining/Audio/Hidden.Hidden")
    (`AudioComponent.Play` _audio 0.0)))

(fn `Play Widget Anim`
  (params (Widget :type "WidgetComponent Object Reference") (Forward :type Boolean))
  (bind _aswbp_lecture (cast `/Game/FireTraining/Blueprints/Widgets/WBP_Lecture` (`WidgetComponent.GetUserWidgetObject` Widget)))
  (if Forward
    (bind _imageanim (`/Game/FireTraining/Blueprints/Widgets/WBP_Lecture.ImageAnim` _aswbp_lecture))
    (`UserWidget.PlayAnimationForward` _aswbp_lecture _imageanim 1.0 false)
    (else
      (`UserWidget.PlayAnimationReverse` _aswbp_lecture _imageanim 1.0 false))))

(fn `Set Lecture Image`
  (params (Widget :type "WidgetComponent Object Reference") (Image :type "Texture2D Object Reference"))
  (bind _aswbp_lecture (cast `/Game/FireTraining/Blueprints/Widgets/WBP_Lecture` (`WidgetComponent.GetUserWidgetObject` Widget)))
  (`Image.SetBrushFromTexture` (`/Game/FireTraining/Blueprints/Widgets/WBP_Lecture.Image_24` _aswbp_lecture) Image true))

(fn `UserConstructionScript`)