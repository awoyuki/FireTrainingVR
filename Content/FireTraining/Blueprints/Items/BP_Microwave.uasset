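; Burning microwave fire hazard for VR fire training, toggling particles, audio and mesh collision with its fire state.
; Its DangerZone shows a warning widget to nearby players.
; Touching the mesh with a hand burns the player, triggering fail notice, haptics, camera fade and return to Lobby.
; Extinguishing is blocked while an assigned BP_Switch is on; otherwise foam warns of wrong extinguisher, while powder and CO2 call OnHitBehaviour.
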(event `self.ReceiveBeginPlay`
  (`parent.ReceiveBeginPlay`)
  (`self.Active Fire On Sample`))

(event `self.Active Fire On Sample`
  (`parent.Active Fire On Sample`)
  (`ParticleSystemComponent.BeginTrails` (`self.ParticleSystem`) "None" "None" "ETrailWidthMode_FromFirst" 0.0)
  (`AudioComponent.Play` (`self.Audio`) 0.0)
  (`PrimitiveComponent.SetCollisionEnabled` (`self.StaticMeshComponent`) "QueryAndPhysics"))

(event `self.Deactive Fire On Sample`
  (`parent.Deactive Fire On Sample`)
  (`ParticleSystemComponent.EndTrails` (`self.ParticleSystem`))
  (`AudioComponent.Stop` (`self.Audio`))
  (`PrimitiveComponent.SetCollisionEnabled` (`self.StaticMeshComponent`) "NoCollision")
  (`self.On Extinghuised`))

(event `self.DangerZone.OnComponentBeginOverlap`
  (params (OverlappedComponent :type "PrimitiveComponent Object Reference") (OtherActor :type "Actor Object Reference") (OtherComp :type "PrimitiveComponent Object Reference") (OtherBodyIndex :type Integer) (bFromSweep :type Boolean) (SweepResult :type "HitResult Structure (by ref)"))
  (bind _asvive_pawn_character (cast `/Game/VRExpansion/Vive/Vive_PawnCharacter` OtherActor))
  (if (and (== OtherComp (`Character.CapsuleComponent` _asvive_pawn_character)) (> (`self.Health`) 0))
    (bind _returnvalue (`/Game/VRExpansion/Vive/Vive_PawnCharacter.Show Notifycation` _asvive_pawn_character "/Game/FireTraining/Blueprints/Widgets/WBP_DangerZone.WBP_DangerZone_C"))))

(event `self.DangerZone.OnComponentEndOverlap`
  (params (OverlappedComponent :type "PrimitiveComponent Object Reference") (OtherActor :type "Actor Object Reference") (OtherComp :type "PrimitiveComponent Object Reference") (OtherBodyIndex :type Integer))
  (bind _asvive_pawn_character (cast `/Game/VRExpansion/Vive/Vive_PawnCharacter` OtherActor))
  (if (and (== OtherComp (`Character.CapsuleComponent` _asvive_pawn_character)) (not (`self.PlayerInjure`)))
    (`/Game/FireTraining/Blueprints/Widgets/WBP_UI.Disable Notifycation` (`/Game/VRExpansion/Vive/Vive_PawnCharacter.As WBP UI` _asvive_pawn_character) (stale `self.DangerZone.OnComponentBeginOverlap` _returnvalue) false)))

(event `self.StaticMeshComponent.OnComponentBeginOverlap`
  (params (OverlappedComponent :type "PrimitiveComponent Object Reference") (OtherActor :type "Actor Object Reference") (OtherComp :type "PrimitiveComponent Object Reference") (OtherBodyIndex :type Integer) (bFromSweep :type Boolean) (SweepResult :type "HitResult Structure (by ref)"))
  (bind _asgrasping_hand (cast `/Game/VRExpansion/Vive/Testing/GraspingHand/GraspingHand` OtherActor))
  (bind _returnvalue (`self.GetOwner` _asgrasping_hand))
  (bind _asvive_pawn_character (cast `/Game/VRExpansion/Vive/Vive_PawnCharacter` _returnvalue))
  (`/Engine/EditorBlueprintResources/StandardMacros.DoOnce` false
    (:`Completed`
      (bind _returnvalue_2 (`/Game/VRExpansion/Vive/Vive_PawnCharacter.Show Notifycation` _asvive_pawn_character "/Game/FireTraining/Blueprints/Widgets/WBP_TaskFail.WBP_TaskFail_C"))
      (bind _aswbp_task_fail (cast `/Game/FireTraining/Blueprints/Widgets/WBP_TaskFail` _returnvalue_2))
      (`TextBlock.SetText` (`/Game/FireTraining/Blueprints/Widgets/WBP_TaskFail.Content` _aswbp_task_fail) "Bạn đã bị bỏng!  \nBạn sẽ được đưa về sảnh chính để trị thương. Hãy cẩn thận và đọc kỹ các lý thuyết trước khi thực hành nhé!")
      (bind _aspc_fire_training (cast `/Game/FireTraining/Framework/PC_FireTraining` (`self.GetOwner` _returnvalue)))
      (`PlayerCameraManager.StartCameraFade` :`self` (`GameplayStatics.GetPlayerCameraManager` (`GameplayStatics.GetPlayerControllerID` _aspc_fire_training)) :`ToAlpha` 1.0 :`Duration` 3.0 :`bShouldFadeAudio` true :`bHoldWhenFinished` true)
      (`PlayerController.PlayHapticEffect` _aspc_fire_training "/Game/FireTraining/Effects/NewHapticFeedbackEffect_Curve.NewHapticFeedbackEffect_Curve" (`GripMotionControllerComponent.GetHandType` (`/Game/VRExpansion/Vive/Testing/GraspingHand/GraspingHand.OwningController` _asgrasping_hand)) 1.0 true)
      (`ParticleSystemComponent.BeginTrails` (`/Game/VRExpansion/Vive/Testing/GraspingHand/GraspingHand.ParticleSystem` _asgrasping_hand) "None" "None" "ETrailWidthMode_FromCentre" 0.0)
      (set `self.PlayerInjure` true)
      (`KismetSystemLibrary.Delay` 3.0)
      (`GameplayStatics.OpenLevel` "Lobby"))))

(event `self.Extinguished`
  (params (Type :type "/Game/FireTraining/Blueprints/Enums/E_Fireextinguisher Enum" :default "NewEnumerator0") (Target :type "Actor Object Reference"))
  (bind _electricsupply (`self.ElectricSupply`)
    (:`then`
      (bind _asbp_switch (cast `/Game/FireTraining/Blueprints/Items/BP_Switch` _electricsupply))
      (if (`/Game/FireTraining/Blueprints/Items/BP_Switch.IsOn` _asbp_switch)
        (bind _asvive_pawn_character (cast `/Game/VRExpansion/Vive/Vive_PawnCharacter` (`self.GetOwner` Target)))
        (`/Engine/EditorBlueprintResources/StandardMacros.DoOnce` false
          (:`Completed`
            (bind _returnvalue (`/Game/VRExpansion/Vive/Vive_PawnCharacter.Show Notifycation` _asvive_pawn_character "/Game/FireTraining/Blueprints/Widgets/WBP_TaskFail.WBP_TaskFail_C"))
            (add `/Game/FireTraining/Blueprints/Widgets/WBP_UI.On Disable Notify` (`/Game/VRExpansion/Vive/Vive_PawnCharacter.As WBP UI` _asvive_pawn_character) (delegate `CustomEvent_1`))
            (bind _aswbp_warning (cast `/Game/FireTraining/Blueprints/Widgets/WBP_Warning` _returnvalue))
            (`TextBlock.SetText` (`/Game/FireTraining/Blueprints/Widgets/WBP_Warning.Content` _aswbp_warning) "Bạn chưa tắt nguồn điện trước khi dập tắt đám cháy! ")))
        (else
          (switch `/Game/FireTraining/Blueprints/Enums/E_Fireextinguisher` Type :!label _label
            (:`NewEnumerator0`
              (bind _asvive_pawn_character_2 (cast `/Game/VRExpansion/Vive/Vive_PawnCharacter` Target))
              (`/Engine/EditorBlueprintResources/StandardMacros.DoOnce` false :!label _label_2
                (:`Completed`
                  (bind _returnvalue_2 (`/Game/VRExpansion/Vive/Vive_PawnCharacter.Show Notifycation` _asvive_pawn_character_2 "/Game/FireTraining/Blueprints/Widgets/WBP_Warning.WBP_Warning_C"))
                  (add `/Game/FireTraining/Blueprints/Widgets/WBP_UI.On Disable Notify` (`/Game/VRExpansion/Vive/Vive_PawnCharacter.As WBP UI` _asvive_pawn_character_2) (delegate `CustomEvent`))
                  (bind _aswbp_warning_2 (cast `/Game/FireTraining/Blueprints/Widgets/WBP_Warning` _returnvalue_2))
                  (`TextBlock.SetText` (`/Game/FireTraining/Blueprints/Widgets/WBP_Warning.Content` _aswbp_warning_2) "Bạn đã sử dụng sai bình xịt!  \nVui lòng sử dụng bình xịt loại khác!"))))
            (:`NewEnumerator1`
              (`self.On Hit Behaviour` :!label _label_3))
            (:`NewEnumerator2`
              (goto _label_3))))))
    (:`else`
      (goto _label))))

(event `CustomEvent_1`
  (params (Removed :type "Widget Object Reference"))
  (if (== (stale `self.Extinguished` _returnvalue) Removed)
    (remove `/Game/FireTraining/Blueprints/Widgets/WBP_UI.On Disable Notify` (`/Game/VRExpansion/Vive/Vive_PawnCharacter.As WBP UI` (stale `self.Extinguished` _asvive_pawn_character)) (delegate `CustomEvent_1`))))

(event `CustomEvent`
  (params (Removed :type "Widget Object Reference"))
  (if (== (stale `self.Extinguished` _returnvalue_2) Removed)
    (remove `/Game/FireTraining/Blueprints/Widgets/WBP_UI.On Disable Notify` (`/Game/VRExpansion/Vive/Vive_PawnCharacter.As WBP UI` (stale `self.Extinguished` _asvive_pawn_character_2)) (delegate `CustomEvent`))
    (goto _label_2 :!via `Reset`)))

(fn `UserConstructionScript`
  (`parent.UserConstructionScript`))