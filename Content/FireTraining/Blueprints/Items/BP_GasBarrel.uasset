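; BP_GasBarrel is a burning gas barrel for VR fire training that accepts only powder extinguishers.
; It extends parent fire activation and deactivation with particle trails and audio.
; Powder triggers the hit behaviour, while foam and CO2 show a Vietnamese warning pointing to dry powder.
; While Health remains, hands entering the box get burn trails, looping haptics and a burn warning, all cleared on exit.
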(event `/Game/FireTraining/Blueprints/Interfaces/BPI_Sample.Active Fire On Sample`
  (`parent.Active Fire On Sample`)
  (`ParticleSystemComponent.BeginTrails` (`self.ParticleSystem`) "None" "None" "ETrailWidthMode_FromFirst" 0.0)
  (`AudioComponent.Play` (`self.Audio`) 0.0))

(event `/Game/FireTraining/Blueprints/Interfaces/BPI_Sample.Deactive Fire On Sample`
  (`parent.Deactive Fire On Sample`)
  (`ParticleSystemComponent.EndTrails` (`self.ParticleSystem`))
  (`AudioComponent.Stop` (`self.Audio`)))

(event `self.Extinguished`
  (params (Type :type "/Game/FireTraining/Blueprints/Enums/E_Fireextinguisher Enum" :default "NewEnumerator0") (Target :type "Actor Object Reference"))
  (switch `/Game/FireTraining/Blueprints/Enums/E_Fireextinguisher` Type
    (:`NewEnumerator0`
      (`self.Warning` Target "- Bình dạng bột khô Powder" :!label _label))
    (:`NewEnumerator1`
      (`self.On Hit Behaviour`))
    (:`NewEnumerator2`
      (goto _label))))

(event `self.Box.OnComponentBeginOverlap`
  (params (OverlappedComponent :type "PrimitiveComponent Object Reference") (OtherActor :type "Actor Object Reference") (OtherComp :type "PrimitiveComponent Object Reference") (OtherBodyIndex :type Integer) (bFromSweep :type Boolean) (SweepResult :type "HitResult Structure (by ref)"))
  (if (> (`self.Health`) 0)
    (bind _asgrasping_hand (cast `/Game/VRExpansion/Vive/Testing/GraspingHand/GraspingHand` OtherActor))
    (`ParticleSystemComponent.BeginTrails` (`/Game/VRExpansion/Vive/Testing/GraspingHand/GraspingHand.ParticleSystem` _asgrasping_hand) "None" "None" "ETrailWidthMode_FromCentre" 0.0)
    (bind _asvive_pawn_character (cast `/Game/VRExpansion/Vive/Vive_PawnCharacter` (`self.GetOwner` _asgrasping_hand)))
    (bind _aspc_fire_training (cast `/Game/FireTraining/Framework/PC_FireTraining` (`self.GetOwner` _asvive_pawn_character)))
    (`PlayerController.PlayHapticEffect` _aspc_fire_training "/Game/FireTraining/Effects/NewHapticFeedbackEffect_Curve.NewHapticFeedbackEffect_Curve" (`GripMotionControllerComponent.GetHandType` (`/Game/VRExpansion/Vive/Testing/GraspingHand/GraspingHand.OwningController` _asgrasping_hand)) 1.0 true)
    (bind _returnvalue (`/Game/VRExpansion/Vive/Vive_PawnCharacter.Show Notifycation` _asvive_pawn_character "/Game/FireTraining/Blueprints/Widgets/WBP_Warning.WBP_Warning_C"))
    (bind _aswbp_warning (cast `/Game/FireTraining/Blueprints/Widgets/WBP_Warning` _returnvalue))
    (`TextBlock.SetText` (`/Game/FireTraining/Blueprints/Widgets/WBP_Warning.Content` _aswbp_warning) "Bạn đã bị bỏng! \nHãy cẩn thận trước đám cháy!")))

(event `self.Box.OnComponentEndOverlap`
  (params (OverlappedComponent :type "PrimitiveComponent Object Reference") (OtherActor :type "Actor Object Reference") (OtherComp :type "PrimitiveComponent Object Reference") (OtherBodyIndex :type Integer))
  (bind _asgrasping_hand (cast `/Game/VRExpansion/Vive/Testing/GraspingHand/GraspingHand` OtherActor))
  (`ParticleSystemComponent.EndTrails` (`/Game/VRExpansion/Vive/Testing/GraspingHand/GraspingHand.ParticleSystem` _asgrasping_hand))
  (bind _asvive_pawn_character (cast `/Game/VRExpansion/Vive/Vive_PawnCharacter` (`self.GetOwner` _asgrasping_hand)))
  (bind _aspc_fire_training (cast `/Game/FireTraining/Framework/PC_FireTraining` (`self.GetOwner` _asvive_pawn_character)))
  (`PlayerController.StopHapticEffect` _aspc_fire_training (`GripMotionControllerComponent.GetHandType` (`/Game/VRExpansion/Vive/Testing/GraspingHand/GraspingHand.OwningController` _asgrasping_hand)))
  (`/Game/FireTraining/Blueprints/Widgets/WBP_UI.Disable Notifycation` (`/Game/VRExpansion/Vive/Vive_PawnCharacter.As WBP UI` _asvive_pawn_character) null true))

(fn `UserConstructionScript`)