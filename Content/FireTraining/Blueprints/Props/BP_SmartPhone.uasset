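; BP_SmartPhone is a smartphone prop for the fire training game that plays audio.
; Each use toggles its Audio component between playing from the start and stopping.
; ChangeVolume fades between a loud level with high attenuation settings and a normal level with low attenuation settings, using a logarithmic curve.
; Gripping the phone takes the same path as the quieter setting.
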(event `VRGripInterface.OnUsed`
  (bind _audio (`self.Audio`))
  (`/Engine/EditorBlueprintResources/StandardMacros.FlipFlop`
    (:`A`
      (`AudioComponent.Play` _audio 0.0))
    (:`B`
      (`AudioComponent.Stop` _audio))))

(event `Change Volume`
  (params (Louder :type Boolean))
  (if Louder
    (`AudioComponent.AdjustVolume` (`self.Audio`) 1.0 4.0 "Logarithmic")
    (`AudioComponent.AdjustAttenuation` (`self.Audio`) (`self.In Attenuation Settings High`))
    (else
      (`AudioComponent.AdjustVolume` (`self.Audio`) 1.0 1.0 "Logarithmic" :!label _label)
      (`AudioComponent.AdjustAttenuation` (`self.Audio`) (`self.In Attenuation Settings Low`)))))

(event `VRGripInterface.OnGrip`
  (params (GrippingController :type "GripMotionControllerComponent Object Reference") (GripInformation :type "BPActorGripInformation Structure (by ref)"))
  (goto _label))

(fn `UserConstructionScript`)