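; BP_VendingMachineSnacker is a vending machine prop that dispenses a random snack when a GraspingHand overlaps its trigger box.
; It spawns a BP_Item at the Snack transform, gives it a random mesh from PropLists, enables physics and applies a small upward impulse.
; An Active flag with a one-second delay acts as a cooldown between dispenses.
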(event `self.Box.OnComponentBeginOverlap`
  (params (OverlappedComponent :type "PrimitiveComponent Object Reference") (OtherActor :type "Actor Object Reference") (OtherComp :type "PrimitiveComponent Object Reference") (OtherBodyIndex :type Integer) (bFromSweep :type Boolean) (SweepResult :type "HitResult Structure (by ref)"))
  (if (not (`self.Active`))
    (cast `/Game/VRExpansion/Vive/Testing/GraspingHand/GraspingHand` OtherActor)
    (`self.Spawn Props`)
    (set `self.Active` true)
    (`KismetSystemLibrary.Delay` 1.0)
    (set `self.Active` false)))

(fn `Spawn Props`
  (bind _returnvalue (`|SpawnActorFromClass` "/Game/FireTraining/Blueprints/Items/BP_Item.BP_Item_C" (`SceneComponent.K2_GetComponentToWorld` (`self.Snack`)) "AlwaysSpawn" "OverrideRootScale" null null))
  (bind _staticmeshcomponent (`StaticMeshActor.StaticMeshComponent` _returnvalue))
  (bind _returnvalue_2 (`StaticMeshComponent.SetStaticMesh` _staticmeshcomponent (`KismetArrayLibrary.Array_Random` (`self.PropLists`))))
  (`PrimitiveComponent.SetSimulatePhysics` _staticmeshcomponent _returnvalue_2)
  (`PrimitiveComponent.AddImpulse` _staticmeshcomponent (0.0 0.0 50.0) "None" false))

(fn `UserConstructionScript`)