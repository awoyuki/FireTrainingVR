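; Dock radio prop that accepts a BP_SmartPhone and controls its volume.
; When the phone overlaps the Box, the first holding motion controller drops it and it snaps to the mesh's PhoneBase socket.
; Docking applies the current loudness flag to the phone, and OnUsed toggles that flag while the stored phone reference is valid.
; The phone reference is never cleared here.
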(event `self.Box.OnComponentBeginOverlap`
  (params (OverlappedComponent :type "PrimitiveComponent Object Reference") (OtherActor :type "Actor Object Reference") (OtherComp :type "PrimitiveComponent Object Reference") (OtherBodyIndex :type Integer) (bFromSweep :type Boolean) (SweepResult :type "HitResult Structure (by ref)"))
  (bind _asbp_smart_phone (cast `/Game/FireTraining/Blueprints/Props/BP_SmartPhone` OtherActor))
  (bind _output_get (set `self.As BP Smart Phone` _asbp_smart_phone))
  (bind _holdingcontrollers (`VRGripInterface.IsHeld` _output_get))
  (bind (_holdingcontroller _gripid) (break `BPGripPair` (`|GetArrayItem` _holdingcontrollers)))
  (`GripMotionControllerComponent.DropObject` _holdingcontroller _output_get _gripid false (0.0 0.0 0.0) (0.0 0.0 0.0))
  (`self.K2_AttachToComponent` _output_get (`self.StaticMeshComponent`) "PhoneBase" "SnapToTarget" "SnapToTarget" "KeepWorld" true)
  (`/Game/FireTraining/Blueprints/Props/BP_SmartPhone.Change Volume` _output_get (`self.Lounder`)))

(event `VRGripInterface.OnUsed`
  (bind _as_bp_smart_phone (`self.As BP Smart Phone`))
  (`/Engine/EditorBlueprintResources/StandardMacros.IsValid` _as_bp_smart_phone
    (:`Is Valid`
      (bind _output_get (set `self.Lounder` (not (`self.Lounder`))))
      (`/Game/FireTraining/Blueprints/Props/BP_SmartPhone.Change Volume` _as_bp_smart_phone _output_get))))

(fn `UserConstructionScript`)