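; BP_FlammableObject is a prop for fire training that reacts to fire and extinguisher events on a hit component.
; OnFire calls BeginTrails on the particle system children of the hit component.
; Each OnExtinguisher event runs ReduceDamage, which counts Damage down by one until it is already at or below zero.
; Only then does it clamp Damage to zero and call EndTrails on those particle children.
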(event `On Fire`
  (params (`Component Hit` :type "SceneComponent Object Reference"))
  (for _array_element (`SceneComponent.GetChildrenComponents` `Component Hit` false)
    (bind _asparticle_system_component (cast `ParticleSystemComponent` _array_element))
    (`ParticleSystemComponent.BeginTrails` _asparticle_system_component "None" "None" "ETrailWidthMode_FromCentre" 0.0)))

(event `On Extinguisher`
  (params (`Component Hit` :type "SceneComponent Object Reference"))
  (bind _extinged (`self.Reduce Damage`))
  (if _extinged
    (for _array_element (`SceneComponent.GetChildrenComponents` `Component Hit` false)
      (bind _asparticle_system_component (cast `ParticleSystemComponent` _array_element))
      (`ParticleSystemComponent.EndTrails` _asparticle_system_component))))

(fn `Reduce Damage`
  (returns (Extinged :type Boolean))
  (bind _damage (`self.Damage`))
  (if (<= _damage 0.0)
    (set `self.Damage` 0.0)
    (return true)
    (else
      (`/Engine/EditorBlueprintResources/StandardMacros.DecrementFloat` _damage
        (:`  `
          (return false))))))

(fn `UserConstructionScript`)