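; Physical VR push-button mesh component that depresses under overlapping grippable objects or grasping hands and reports its state through a ButtonPressed event.
; Overlap enables tick, which tracks the pusher's depth in parent-relative space, clamps travel, then springs back and disables itself on release.
; Passing the toggle depth flips state once per touch, rate-limited by a minimum interval, while press-type buttons follow depth.
; A dynamic material shows on/off color.
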(event `self.ReceiveBeginPlay`
  (add `self.OnComponentBeginOverlap` (delegate `OnComponentBeginOverlap_Event_0`))
  (add `self.OnComponentEndOverlap` (delegate `OnComponentEndOverlap_Event_0`))
  (bind _returnvalue (`self.CreateDynamicMaterialInstance` 0 (`self.GetMaterial` 0)))
  (set `self.MatInstance` _returnvalue)
  (`self.SetColor`)
  (set `self.InitialRelativeTransform` (`self.GetRelativeTransform`)))

(event `OnComponentBeginOverlap_Event_0` :!signature `self.OnComponentBeginOverlap`
  (params (OverlappedComponent :type "PrimitiveComponent Object Reference") (OtherActor :type "Actor Object Reference") (OtherComp :type "PrimitiveComponent Object Reference") (OtherBodyIndex :type Integer) (bFromSweep :type Boolean) (SweepResult :type "HitResult Structure (by ref)"))
  (bind _currenttransform (`self.GetCurrentTransform`))
  (bind (_returnvalue_x _returnvalue_y _returnvalue_z) (`KismetMathLibrary.BreakVector` (`KismetMathLibrary.InverseTransformLocation` _currenttransform (`self.K2_GetComponentLocation`))))
  (if (not (`self.bActive`))
    (bind _asgrippable_static_mesh_component (cast `GrippableStaticMeshComponent` OtherComp)
      (:`then`
        (bind (_holdingcontrollers _bisheld) (`VRGripInterface.IsHeld` _asgrippable_static_mesh_component))
        (if _bisheld
          _
          (else
            _))
        (bind _output_get (set `self.CurrentInteractionObject` OtherComp :!label _label))
        (bind (_returnvalue_x_2 _returnvalue_y_2 _returnvalue_z_2) (`KismetMathLibrary.BreakVector` (`KismetMathLibrary.InverseTransformLocation` _currenttransform (`self.K2_GetComponentLocation` _output_get))))
        (set `self.InitialZ` _returnvalue_z_2)
        (set `self.InitialComponentZ` _returnvalue_z)
        (`self.SetComponentTickEnabled` true)
        (set `self.ToggledThisTouch` false)
        (set `self.bLerping` false)
        (set `self.bActive` true))
      (:`CastFailed`
        (cast `OptionalRepStaticMeshComponent` OtherComp
          (:`then`
            (bind _asvrgrip_interface (cast `VRGripInterface` OtherActor))
            (bind (_holdingcontrollers_2 _bisheld_2) (`VRGripInterface.IsHeld` _asvrgrip_interface))
            (if _bisheld_2
              (goto _label)))
          (:`CastFailed`
            (cast `/Game/VRExpansion/Vive/Testing/GraspingHand/GraspingHand` OtherActor)
            (goto _label)))))))

(event `OnComponentEndOverlap_Event_0` :!signature `self.OnComponentEndOverlap`
  (params (OverlappedComponent :type "PrimitiveComponent Object Reference") (OtherActor :type "Actor Object Reference") (OtherComp :type "PrimitiveComponent Object Reference") (OtherBodyIndex :type Integer))
  (if (`self.bActive`)
    (if (== (`self.CurrentInteractionObject`) OtherComp)
      (set `self.bActive` false))))

(event `self.ReceiveTick`
  (params (DeltaSeconds :type "Float (single-precision)"))
  (bind _initialrelativetransform_location (`KismetMathLibrary.BreakTransform` (`self.InitialRelativeTransform`)))
  (bind _depressdistance (`self.DepressDistance`))
  (bind _returnvalue (`KismetMathLibrary.VInterpTo_Constant` (`self.RelativeLocation`) _initialrelativetransform_location (`GameplayStatics.GetWorldDeltaSeconds`) (`self.DepressSpeed`)))
  (bind (_returnvalue_x _returnvalue_y _returnvalue_z) (`KismetMathLibrary.BreakVector` (`KismetMathLibrary.InverseTransformLocation` (`self.InitialRelativeTransform`) (`self.RelativeLocation`))))
  (bind (_returnvalue_x_2 _returnvalue_y_2 _returnvalue_z_2) (`KismetMathLibrary.BreakVector` (`KismetMathLibrary.InverseTransformLocation` (`self.GetCurrentTransform`) (`self.K2_GetComponentLocation` (`self.CurrentInteractionObject`)))))
  (bind _returnvalue_2 (<= _returnvalue_z (+ (* (`self.SwitchToggleDepth`) -1.0) 0.001)))
  (bind _returnvalue_3 (`KismetMathLibrary.FClamp` (- (`self.InitialZ`) _returnvalue_z_2) 0.0 _depressdistance))
  (bind _returnvalue_4 (`KismetMathLibrary.FClamp` (+ (`self.InitialComponentZ`) (* _returnvalue_3 -1.0)) (* _depressdistance -1.0) 0.0))
  (`|ExecutionSequence`
    (:`then_1`
      (if (`self.bActive`)
        (if (> _returnvalue_3 0.0)
          (`self.K2_SetRelativeLocation` (`KismetMathLibrary.TransformLocation` (`self.InitialRelativeTransform`) (`KismetMathLibrary.MakeVector` 0.0 0.0 _returnvalue_4)))
          (if (and (<= _returnvalue_4 (+ (* (`self.SwitchToggleDepth`) -1.0) 0.001)) (not (`self.ToggledThisTouch`)))
            (bind _setbutton (`self.CheckForButtonPress` (not (`self.ButtonState`))))
            (if _setbutton
              (`self.SetColor`)
              (set `self.ToggledThisTouch` true))))
        (else
          ;[1 1 1] This fixes the overlap / tick out of sync issue, running the clear in tick to ensure its not trying to pull the current interaction object when its invalid.
          (if (not (`self.bLerping`))
            (set `self.CurrentInteractionObject` null)
            (set `self.bLerping` true)))))
    (:`then_2`
      (if (`self.bLerping`)
        ;[1 1 1] Interp back to position
        (`self.K2_SetRelativeLocation` _returnvalue)
        (if (== _returnvalue (0.0 0.0 0.0))
          (set `self.bLerping` false)
          (`self.SetComponentTickEnabled` false))))
    (:`then_3`
      ;[1 1 1] Set color for non toggle button
      (switch `/Game/VRExpansion/Vive/Testing/Button/EButtonType` (`self.ButtonType`)
        (:`NewEnumerator1`
          (if (!= _returnvalue_2 (`self.ButtonState`))
            (bind _output_get (set `self.ButtonState` _returnvalue_2))
            (`self.CheckForButtonPress` _output_get)
            (`self.SetColor`)))))))

(fn `CheckForButtonPress`
  (params (StateValue :type Boolean))
  (returns (SetButton :type Boolean))
  (if (>= (`KismetMathLibrary.GetTotalSeconds` (- (`KismetMathLibrary.Now`) (`self.LastToggleTime`))) (`self.MinTimeBetweenToggles`))
    (bind _output_get (set `self.ButtonState` StateValue))
    (`self.ButtonPressed` _output_get)
    (set `self.LastToggleTime` (`KismetMathLibrary.Now`))
    (return true)
    (else
      (return false))))

(fn `GetCurrentTransform`
  (returns (CurrentTransform :type "Transform Structure"))
  (bind _returnvalue (`self.GetAttachParent`))
  (`/Engine/EditorBlueprintResources/StandardMacros.IsValid` _returnvalue
    (:`Is Valid`
      (return (`KismetMathLibrary.ComposeTransforms` (`self.InitialRelativeTransform`) (`self.K2_GetComponentToWorld` _returnvalue))))
    (:`Is Not Valid`
      (return (`self.InitialRelativeTransform`)))))

(fn `SetColor`
  (bind _matinstance (`self.MatInstance`))
  (if (`self.ButtonState`)
    (`MaterialInstanceDynamic.SetVectorParameterValue` _matinstance "ButtonColor" (`self.OnColor`))
    (else
      (`MaterialInstanceDynamic.SetVectorParameterValue` _matinstance "ButtonColor" (`self.OffColor`)))))